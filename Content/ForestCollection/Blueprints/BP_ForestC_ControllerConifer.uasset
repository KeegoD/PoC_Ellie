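; Controller actor for the Forest Collection conifer scene that sets ground wetness and scene lighting from its variables.
; It writes the wetness multiplier and power into the MPC_ForestC_General material parameter collection and sets SkyLight and DirectionalLight intensities.
; The same logic runs in both the construction script, so edits update in the editor, and BeginPlay, so values apply at game start.
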(event EventBeginPlay
  (Rendering|Material|SetScalarParameterValue "/Game/ForestCollection/Blueprints/MPC_ForestC_General.MPC_ForestC_General" "FTC_Ground_WetnessMultipler" (Variables|Ground|GetFTC_GroundWetnessMultiplier) :!class /Script/Engine.KismetMaterialLibrary)
  (Rendering|Material|SetScalarParameterValue "/Game/ForestCollection/Blueprints/MPC_ForestC_General.MPC_ForestC_General" "FTC_Ground_WetnessPower" (Variables|Ground|GetFTC_GroundWetnessPower) :!class /Script/Engine.KismetMaterialLibrary)
  (Rendering|Components|Light|SetIntensity (Variables|Default|GetSkyLight) (Variables|Lighting|GetFTC_SkyIntensity))
  (Rendering|Components|Light|SetIntensity (Variables|Default|GetDirectionalLight) (Variables|Lighting|GetFTC_SunIntensity)))

(event EventActorBeginOverlap
  (params (OtherActor :type Actor%20Object%20Reference)))

(event EventTick
  (params (DeltaSeconds :type Float%20%28single-precision%29)))

(fn ConstructionScript
  (Rendering|Material|SetScalarParameterValue "/Game/ForestCollection/Blueprints/MPC_ForestC_General.MPC_ForestC_General" "FTC_Ground_WetnessMultipler" (Variables|Ground|GetFTC_GroundWetnessMultiplier) :!class /Script/Engine.KismetMaterialLibrary)
  (Rendering|Material|SetScalarParameterValue "/Game/ForestCollection/Blueprints/MPC_ForestC_General.MPC_ForestC_General" "FTC_Ground_WetnessPower" (Variables|Ground|GetFTC_GroundWetnessPower) :!class /Script/Engine.KismetMaterialLibrary)
  (Rendering|Components|Light|SetIntensity (Variables|Default|GetSkyLight) (Variables|Lighting|GetFTC_SkyIntensity))
  (Rendering|Components|Light|SetIntensity (Variables|Default|GetDirectionalLight) (Variables|Lighting|GetFTC_SunIntensity)))